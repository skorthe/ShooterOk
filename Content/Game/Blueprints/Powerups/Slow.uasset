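; Slow powerup pickup that spins in place and calls the player character's Speed function with a fixed value on overlap.
; It then teleports far below its stored start location and returns after a short delay, acting as a respawn without destroying the actor.
; Both teleports build the transform from location alone, so rotation and scale reset to defaults.
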(event EventBeginPlay
  (Variables|Default|SetOriginal%20Vector_0 (Transformation|GetActorLocation)))

(event Collision|EventActorBeginOverlap
  (params (OtherActor :type Actor%20Object%20Reference))
  (bind _asbp_player_character (Utilities|Casting|CastToBP_PlayerCharacter OtherActor))
  (Default|Speed _asbp_player_character 3e+02)
  (Transformation|SetActorTransform (Math|Conversions|ToTransform(Vector) (- (Variables|Default|GetOriginal%20Vector_0) "0,0,1000.000000")) false true)
  (Utilities|FlowControl|Delay 5.0)
  (Transformation|SetActorTransform (Math|Conversions|ToTransform(Vector) (Variables|Default|GetOriginal%20Vector_0)) false true))

(event EventTick
  (params (DeltaSeconds :type Float%20%28single-precision%29))
  (Transformation|AddActorLocalRotation (Math|Rotator|MakeRotator 0.0 0.0 (* DeltaSeconds (Variables|Default|GetRotation))) false false))

(fn ConstructionScript
  (|CallParentFunction))