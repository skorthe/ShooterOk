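; BP_Shotgun is the shotgun weapon, which registers itself in the player's hotbar when touched.
; The construction script sets its stats as a semi-automatic, multi-round-per-shot gun before calling the parent construction script.
; When BP_PlayerCharacter overlaps its Collision component, it writes itself into a fixed hotbar slot (index 2).
; No firing, reloading or pickup hiding is implemented in this Blueprint.
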(event OnComponentBeginOverlap(Collision)
  (params (OverlappedComponent :type Primitive%20Component%20Object%20Reference) (OtherActor :type Actor%20Object%20Reference) (OtherComp :type Primitive%20Component%20Object%20Reference) (OtherBodyIndex :type Integer) (bFromSweep :type Boolean) (SweepResult :type Hit%20Result%20Structure%20%28by%20ref%29))
  (bind _asbp_player_character (Utilities|Casting|CastToBP_PlayerCharacter OtherActor))
  (Utilities|Array|SetArrayElem (Variables|/Game/Game/Blueprints/Player/BP_PlayerCharacter.BP_PlayerCharacter_C|GetHotbar _asbp_player_character) 2 self))

(event EventBeginPlay
  (|CallParentFunction) ; This node is disabled and will not be called.\nDrag off pins to build functionality.
)

(event Collision|EventActorBeginOverlap
  (params (OtherActor :type Actor%20Object%20Reference))
  (|CallParentFunction OtherActor) ; This node is disabled and will not be called.\nDrag off pins to build functionality.
)

(fn ConstructionScript
  (Variables|Default|SetDamage 3e+01)
  (Variables|Default|SetSpread 5.0)
  (Variables|Default|SetRate%20Of%20Fire 0.0)
  (Variables|Default|SetRate%20Of%20Spam 1.0)
  (Variables|Default|SetReload%20Time 0.0)
  (Variables|Default|SetRounds%20Per%20Shot 5)
  (Variables|Default|SetCurrent%20Mag%20Ammo 10)
  (Variables|Default|SetMag%20Capacity 30)
  (Variables|Default|SetWeapon%20Name "Shotgun")
  (Variables|Default|SetAutomatic%20Weapon? false)
  (|CallParentFunction))