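; Base weapon Blueprint providing hitscan firing functions for shotgun, SMG and pistol, with an empty Fire event.
; Each traces rounds from the player's camera within a random spread cone while left click is held, spawning explosion effects on hits.
; Timers re-invoke firing: SMG loops, while shotgun and pistol both schedule Shotgun Rounds once and set Fired on hits.
; Only pistol hits deduct magazine ammo; no damage is applied.
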(event Custom|Fire)

(event EventBeginPlay)

(event Collision|EventActorBeginOverlap
  (params (OtherActor :type Actor%20Object%20Reference)))

(event EventTick
  (params (DeltaSeconds :type Float%20%28single-precision%29)))

(fn ConstructionScript)

(fn PSpread
  (params (Input%20Trace :type Vector))
  (bind (_x _y _z) (Math|Vector|BreakVector Input%20Trace))
  (bind _spread (Variables|Default|GetSpread))
  (bind _returnvalue (* _spread -1.0))
  (return (Math|Vector|MakeVector (+ _x (Math|Random|RandomFloatinRange _returnvalue _spread)) (+ _y (Math|Random|RandomFloatinRange _returnvalue _spread)) (+ _z (Math|Random|RandomFloatinRange _returnvalue _spread)))))

(fn ShotgunRounds
  (bind _returnvalue (Game|GetPlayerCharacter 0))
  ;[1 1 1] Sets rate of fire for automatic weapons, and loops if weapon is automatic
  (if (not (Variables|Default|GetFired?))
    (bind _returnvalue_2 (Utilities|Time|SetTimerbyFunctionName 0 "Shotgun Rounds" (Variables|Default|GetRate%20Of%20Fire)))
    ;[1 1 1] Code that makes weapons shoot out multiple rounds per shot
    (for _index (range 1 (Variables|Default|GetRounds%20Per%20Shot))
      ;[1 1 1] Stops automatic weapons when the player releases left click
      (bind _asbp_player_character (Utilities|Casting|CastToBP_PlayerCharacter _returnvalue))
      (Variables|Default|SetCharacter%20Reference 0)
      (if (Variables|/Game/Game/Blueprints/Player/BP_PlayerCharacter.BP_PlayerCharacter_C|GetLeftClickDown? _asbp_player_character)
        ;[1 1 1] makes projectiles ignore friendly AI and player
        (bind _asbp_player_character_2 (Utilities|Casting|CastToBP_PlayerCharacter _returnvalue))
        (Variables|Default|SetCharacters%20To%20Ignore (Utilities|Array|MakeArray _asbp_player_character_2))
        ;[1 1 1] Hitscan (Line trace) starts at First person camera world location (Shotgun cone logic)
        (bind _asbp_player_character_3 (Utilities|Casting|CastToBP_PlayerCharacter (Game|GetPlayerCharacter 0)))
        (bind (_outhit _returnvalue_3) (Collision|LineTraceByChannel (Transformation|GetWorldLocation (Variables|/Game/Game/Blueprints/Player/BP_PlayerCharacter.BP_PlayerCharacter_C|GetFirstPersonCamera _asbp_player_character_3)) (+ (Transformation|GetWorldLocation (Variables|/Game/Game/Blueprints/Player/BP_PlayerCharacter.BP_PlayerCharacter_C|GetFirstPersonCamera _asbp_player_character_3)) (* (Math|Random|RandomUnitVectorinConeinDegrees (Math|Vector|GetForwardVector (Variables|/Game/Game/Blueprints/Player/BP_PlayerCharacter.BP_PlayerCharacter_C|GetFirstPersonCamera _asbp_player_character_3)) (Variables|Default|GetSpread)) (Math|Conversions|ToVector(Float) 1e+04))) "TraceTypeQuery1" false (Variables|Default|GetCharacters%20To%20Ignore) "ForDuration"))
        (if _returnvalue_3
          (Effects|SpawnEmitteratLocation "/Game/StarterContent/Particles/P_Explosion.P_Explosion" (.Location (Collision|BreakHitResult _outhit)))
          (Variables|Default|SetFired? true))
        (else
          (Utilities|Time|ClearandInvalidateTimerbyHandle _returnvalue_2))))))

(fn SMGRounds
  (bind _returnvalue (Game|GetPlayerCharacter 0))
  ;[1 1 1] Sets rate of fire for automatic weapons, and loops if weapon is automatic
  (if (not (Variables|Default|GetFired?))
    (bind _returnvalue_2 (Utilities|Time|SetTimerbyFunctionName 0 "SMG Rounds" (Variables|Default|GetRate%20Of%20Fire) true))
    ;[1 1 1] Code that makes weapons shoot out multiple rounds per shot
    (for _index (range 1 (Variables|Default|GetRounds%20Per%20Shot))
      ;[1 1 1] Stops automatic weapons when the player releases left click
      (bind _asbp_player_character (Utilities|Casting|CastToBP_PlayerCharacter _returnvalue))
      (Variables|Default|SetCharacter%20Reference 0)
      (if (Variables|/Game/Game/Blueprints/Player/BP_PlayerCharacter.BP_PlayerCharacter_C|GetLeftClickDown? _asbp_player_character)
        ;[1 1 1] makes projectiles ignore friendly AI and player
        (bind _asbp_player_character_2 (Utilities|Casting|CastToBP_PlayerCharacter _returnvalue))
        (Variables|Default|SetCharacters%20To%20Ignore (Utilities|Array|MakeArray _asbp_player_character_2))
        ;[1 1 1] Hitscan (Line trace) starts at First person camera world location (Full Auto logic)
        (bind _asbp_player_character_3 (Utilities|Casting|CastToBP_PlayerCharacter (Game|GetPlayerCharacter 0)))
        (bind (_outhit _returnvalue_3) (Collision|LineTraceByChannel (Transformation|GetWorldLocation (Variables|/Game/Game/Blueprints/Player/BP_PlayerCharacter.BP_PlayerCharacter_C|GetFirstPersonCamera _asbp_player_character_3)) (+ (Transformation|GetWorldLocation (Variables|/Game/Game/Blueprints/Player/BP_PlayerCharacter.BP_PlayerCharacter_C|GetFirstPersonCamera _asbp_player_character_3)) (* (Math|Random|RandomUnitVectorinConeinDegrees (Math|Vector|GetForwardVector (Variables|/Game/Game/Blueprints/Player/BP_PlayerCharacter.BP_PlayerCharacter_C|GetFirstPersonCamera _asbp_player_character_3)) (Variables|Default|GetSpread)) (Math|Conversions|ToVector(Float) 1e+04))) "TraceTypeQuery1" false (Variables|Default|GetCharacters%20To%20Ignore) "ForDuration"))
        (if _returnvalue_3
          (Effects|SpawnEmitteratLocation "/Game/StarterContent/Particles/P_Explosion.P_Explosion" (.Location (Collision|BreakHitResult _outhit))))
        (else
          (Utilities|Time|ClearandInvalidateTimerbyHandle _returnvalue_2))))))

(fn PistolRounds
  (bind _returnvalue (Game|GetPlayerCharacter 0))
  ;[1 1 1] Sets rate of fire for automatic weapons, and loops if weapon is automatic
  (if (not (Variables|Default|GetFired?))
    (bind _returnvalue_2 (Utilities|Time|SetTimerbyFunctionName 0 "Shotgun Rounds" (Variables|Default|GetRate%20Of%20Fire)))
    ;[1 1 1] Code that makes weapons shoot out multiple rounds per shot
    (for _index (range 1 (Variables|Default|GetRounds%20Per%20Shot))
      ;[1 1 1] Stops automatic weapons when the player releases left click
      (bind _asbp_player_character (Utilities|Casting|CastToBP_PlayerCharacter _returnvalue))
      (Variables|Default|SetCharacter%20Reference 0)
      (if (Variables|/Game/Game/Blueprints/Player/BP_PlayerCharacter.BP_PlayerCharacter_C|GetLeftClickDown? _asbp_player_character)
        ;[1 1 1] makes projectiles ignore friendly AI and player
        (bind _asbp_player_character_2 (Utilities|Casting|CastToBP_PlayerCharacter _returnvalue))
        (Variables|Default|SetCharacters%20To%20Ignore (Utilities|Array|MakeArray _asbp_player_character_2))
        ;[1 1 1] Hitscan (Line trace) starts at First person camera world location (Shotgun cone logic)
        (bind _asbp_player_character_3 (Utilities|Casting|CastToBP_PlayerCharacter (Game|GetPlayerCharacter 0)))
        (bind (_outhit _returnvalue_3) (Collision|LineTraceByChannel (Transformation|GetWorldLocation (Variables|/Game/Game/Blueprints/Player/BP_PlayerCharacter.BP_PlayerCharacter_C|GetFirstPersonCamera _asbp_player_character_3)) (+ (Transformation|GetWorldLocation (Variables|/Game/Game/Blueprints/Player/BP_PlayerCharacter.BP_PlayerCharacter_C|GetFirstPersonCamera _asbp_player_character_3)) (* (Math|Random|RandomUnitVectorinConeinDegrees (Math|Vector|GetForwardVector (Variables|/Game/Game/Blueprints/Player/BP_PlayerCharacter.BP_PlayerCharacter_C|GetFirstPersonCamera _asbp_player_character_3)) (Variables|Default|GetSpread)) (Math|Conversions|ToVector(Float) 1e+04))) "TraceTypeQuery1" false (Variables|Default|GetCharacters%20To%20Ignore) "ForDuration"))
        (if _returnvalue_3
          (Effects|SpawnEmitteratLocation "/Game/StarterContent/Particles/P_Explosion.P_Explosion" (.Location (Collision|BreakHitResult _outhit)))
          (Variables|Default|SetFired? true)
          (Variables|Default|SetCurrent%20Mag%20Ammo (- (Variables|Default|GetCurrent%20Mag%20Ammo) (Variables|Default|GetRounds%20Per%20Shot))))
        (else
          (Utilities|Time|ClearandInvalidateTimerbyHandle _returnvalue_2))))))