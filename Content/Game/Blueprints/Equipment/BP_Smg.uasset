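; BP_Smg is the SMG weapon Blueprint, an automatic gun defined as a child of a parent weapon class.
; Its Construction Script fills in inherited-style stats for damage, spread, timing, ammo, gun index and name, then calls the parent construction script.
; BeginPlay only forwards to the parent and the overlap event is disabled, so the asset adds no firing logic of its own.
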(event EventBeginPlay
  (|CallParentFunction))

(event Collision|EventActorBeginOverlap
  (params (OtherActor :type Actor%20Object%20Reference))
  (|CallParentFunction OtherActor) ; This node is disabled and will not be called.\nDrag off pins to build functionality.
)

(fn ConstructionScript
  (Variables|Default|SetDamage 5.0)
  (Variables|Default|SetSpread 5.0)
  (Variables|Default|SetRate%20Of%20Fire 0.1)
  (Variables|Default|SetRate%20Of%20Spam 0.0)
  (Variables|Default|SetReload%20Time 0.0)
  (Variables|Default|SetRounds%20Per%20Shot 1)
  (Variables|Default|SetCurrent%20Mag%20Ammo 25)
  (Variables|Default|SetMag%20Capacity 25)
  (Variables|Default|SetReloadable%20Ammo 250)
  (Variables|Default|SetGun%20Index 3)
  (Variables|Default|SetWeapon%20Name "SMG")
  (Variables|Default|SetAutomatic%20Weapon? true)
  (|CallParentFunction))