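; BP_Pistol is a pistol weapon Blueprint that configures a semi-automatic, single-round-per-shot gun.
; Its Construction Script sets the inherited-style weapon stats for damage, spread, fire timing, reload, ammo, gun index and name, then calls the parent's Construction Script.
; The Event Graph holds only disabled default event stubs, so the file adds no runtime logic of its own.
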(event EventBeginPlay
  (|CallParentFunction) ; This node is disabled and will not be called.\nDrag off pins to build functionality.
)

(event Collision|EventActorBeginOverlap
  (params (OtherActor :type Actor%20Object%20Reference))
  (|CallParentFunction OtherActor) ; This node is disabled and will not be called.\nDrag off pins to build functionality.
)

(fn ConstructionScript
  (Variables|Default|SetDamage 5.0)
  (Variables|Default|SetSpread 1.0)
  (Variables|Default|SetRate%20Of%20Fire 0.0)
  (Variables|Default|SetRate%20Of%20Spam 0.1)
  (Variables|Default|SetReload%20Time 0.0)
  (Variables|Default|SetRounds%20Per%20Shot 1)
  (Variables|Default|SetCurrent%20Mag%20Ammo 10)
  (Variables|Default|SetMag%20Capacity 10)
  (Variables|Default|SetReloadable%20Ammo 100)
  (Variables|Default|SetGun%20Index 1)
  (Variables|Default|SetWeapon%20Name "Pistol")
  (Variables|Default|SetAutomatic%20Weapon? false)
  (|CallParentFunction))